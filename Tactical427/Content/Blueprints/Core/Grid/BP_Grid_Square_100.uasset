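; Grid actor that builds a flat tile grid around its location in the construction script using a single instanced static mesh.
; SpawnGrid clears old instances, takes mesh, border material and mesh size from DT_GridShapeData by shape enum, then adds one scaled instance per tile.
; A helper snaps the stored center to tile size and derives the bottom-left start, adjusting for even or odd tile counts.
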(event EventBeginPlay)

(event Collision|EventActorBeginOverlap
  (params (OtherActor :type Actor%20Object%20Reference)))

(event EventTick
  (params (DeltaSeconds :type Float%20%28single-precision%29)))

(fn ConstructionScript
  (CallFunction|SpawnGrid (Transformation|GetActorLocation) (Variables|Default|GetGrid%20Tile%20Size) (Variables|Default|GetGrid%20Tile%20Count) (Variables|Default|GetGrid%20Shape)))

(fn SpawnGrid
  (params (centerLocation :type Vector) (tileSize :type Vector) (tileCount :type Vector%202D%20Structure) (shape :type E_GridShape%20Enum :default "NewEnumerator0"))
  (bind _returnvalue (CallFunction|GetCurrentShapeData))
  (bind (_meshsize _mesh _meshmaterial _flatmesh _flatbordermaterial) (Utilities|Struct|BreakS_GridShapeData _returnvalue))
  (Variables|Default|SetGrid%20Center%20Location centerLocation)
  (Variables|Default|SetGrid%20Tile%20Size tileSize)
  (Variables|Default|SetGrid%20Tile%20Count tileCount)
  (Variables|Default|SetGrid%20Shape shape)
  (CallFunction|DestroyGrid)
  (Components|StaticMesh|SetStaticMesh (Variables|Default|GetInstancedStaticMesh) _flatmesh)
  (Rendering|Material|SetMaterial (Variables|Default|GetInstancedStaticMesh) 0 _flatbordermaterial)
  (bind (_center _bottomleft) (CallFunction|CalculateCenterandButtomLeft))
  (Variables|Default|SetGrid%20Center%20Location _center)
  (Variables|Default|SetgridBottomLeftCornerLocation _bottomleft)
  (for _index (range 0 (- (Math|Float|Round (.x (Variables|Default|GetGrid%20Tile%20Count))) 1))
    (LocalVariables|SetX _index)
    (for _index_2 (range 0 (- (Math|Float|Round (.y (Variables|Default|GetGrid%20Tile%20Count))) 1))
      (LocalVariables|SetY _index_2)
      (LocalVariables|SettileTransform (Math|Transform|MakeTransform (+ (Variables|Default|GetgridBottomLeftCornerLocation) (* (Variables|Default|GetGrid%20Tile%20Size) (Math|Vector|MakeVector (Math|Conversions|ToFloat(Integer) (LocalVariables|GetX)) (Math|Conversions|ToFloat(Integer) (LocalVariables|GetY)) 0.0))) "0, 0, 0" (/ (Variables|Default|GetGrid%20Tile%20Size) (.MeshSize (Utilities|Struct|BreakS_GridShapeData (CallFunction|GetCurrentShapeData))))))
      (Class|InstancedStaticMeshComponent|AddInstanceWorldSpace (Variables|Default|GetInstancedStaticMesh) (LocalVariables|GettileTransform)))))

(fn GetCurrentShapeData
  (bind _grid_shape (Variables|Default|GetGrid%20Shape))
  (bind _returnvalue (Utilities|String|EnumtoString _grid_shape))
  (bind _returnvalue_2 (Utilities|GetDataTableRow "/Game/Blueprints/Core/Grid/GridShapes/DT_GridShapeData.DT_GridShapeData" (Utilities|String|StringToName _returnvalue))
    (:then
      (return _returnvalue_2))
    (:RowNotFound
      (Development|PrintString _returnvalue true true "(R=0.635417,G=0.000000,B=0.005618,A=1.000000)" 5.0))))

(fn DestroyGrid
  (Components|InstancedStaticMesh|ClearInstances (Variables|Default|GetInstancedStaticMesh)))

(fn CalculateCenterandButtomLeft
  (bind _grid_tile_count (Variables|Default|GetGrid%20Tile%20Count))
  (LocalVariables|SetC (CallFunction|SnapVectortoVector (Variables|Default|GetGrid%20Center%20Location) (Variables|Default|GetGrid%20Tile%20Size)))
  (return (LocalVariables|GetC) (- (Variables|Default|GetGrid%20Center%20Location) (Math|Conversions|ToVector(Vector2D) (* (/ (- (Variables|Default|GetGrid%20Tile%20Count) (Math|Vector2D|MakeVector2D (Math|Float|SelectFloat 0.0 1.0 (CallFunction|IsFloatEven (.x _grid_tile_count))) (Math|Float|SelectFloat 0.0 1.0 (CallFunction|IsFloatEven (.y _grid_tile_count))))) 2.0) (Math|Conversions|ToVector2D(Vector) (Variables|Default|GetGrid%20Tile%20Size)))))))