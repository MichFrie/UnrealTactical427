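; Grid actor that builds a flat tile grid from instanced static meshes in its construction script, using configurable shape, tile size and count.
; SpawnGrid clears old instances, applies the shape's mesh and material from a DataTable, then adds a scaled instance per index.
; Helpers snap the center and derive the bottom-left origin for squares and triangles only, compressing and alternately flipping triangle tiles.
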(event EventBeginPlay)

(event Collision|EventActorBeginOverlap
  (params (OtherActor :type Actor%20Object%20Reference)))

(event EventTick
  (params (DeltaSeconds :type Float%20%28single-precision%29)))

(fn ConstructionScript
  (CallFunction|SpawnGrid (Transformation|GetActorLocation) (Variables|Default|GetGrid%20Tile%20Size) (Variables|Default|GetGrid%20Tile%20Count) (Variables|Default|GetGrid%20Shape)))

(fn SpawnGrid
  (params (centerLocation :type Vector) (tileSize :type Vector) (tileCount :type Vector%202D%20Structure) (shape :type E_GridShape%20Enum :default "NewEnumerator0"))
  (bind _returnvalue (CallFunction|GetCurrentShapeData))
  (bind (_meshsize _mesh _meshmaterial _flatmesh _flatbordermaterial) (Utilities|Struct|BreakS_GridShapeData _returnvalue))
  (Variables|Default|SetGrid%20Center%20Location centerLocation)
  (Variables|Default|SetGrid%20Tile%20Size tileSize)
  ;[0.9207 1 0.3926] converts float to int for TileSize
  (Variables|Default|SetGrid%20Tile%20Count (Math|Vector2D|MakeVector2D (Math|Conversions|ToFloat(Integer) (Math|Float|Round (.x tileCount))) (Math|Conversions|ToFloat(Integer) (Math|Float|Round (.y tileCount)))))
  (Variables|Default|SetGrid%20Shape shape)
  ;[0.2797 0.2407 1 1 13] destroys all previous instanced of the grid
  (CallFunction|DestroyGrid)
  ;[1 0.5916 0.5015] sets the type of static mesh (Hexagon, Square, Triangle) via DataTable
  (Components|StaticMesh|SetStaticMesh (Variables|Default|GetInstancedStaticMesh) _flatmesh)
  ;[1 1 1] sets Material for desired static Mesh
  (Rendering|Material|SetMaterial (Variables|Default|GetInstancedStaticMesh) 0 _flatbordermaterial)
  ;[0.4825 1 0.6541 1 13] calculates center and bottom left
  (bind (_center _bottomleft) (CallFunction|CalculateCenterandButtomLeft))
  (Variables|Default|SetGrid%20Center%20Location _center)
  (Variables|Default|SetgridBottomLeftCornerLocation _bottomleft)
  ;[0.6229 1 0.5289 1 13] loops through all tiles and sets the x position of every tile
  (for _index (range 0 (- (Math|Float|Round (.x (Variables|Default|GetGrid%20Tile%20Count))) 1))
    (LocalVariables|SetX _index)
    ;[0.625 0.555 1 1 13] loops through all tiles and sets the x position of every tile
    (for _index_2 (range 0 (- (Math|Float|Round (.y (Variables|Default|GetGrid%20Tile%20Count))) 1))
      (LocalVariables|SetY _index_2)
      ;[1 1 1] X and Y Value = Index
      (LocalVariables|SetIndex (Math|Vector2D|MakeVector2D (Math|Conversions|ToFloat(Integer) (LocalVariables|GetX)) (Math|Conversions|ToFloat(Integer) (LocalVariables|GetY))))
      ;[1 0.5747 0.4542 1 13] sets the transform of every tile
      (LocalVariables|SettileTransform (Math|Transform|MakeTransform (CallFunction|GetTileLocationfromGridIndex (LocalVariables|GetIndex)) (CallFunction|GetTileRotationfromGridIndex (LocalVariables|GetIndex)) (/ (Variables|Default|GetGrid%20Tile%20Size) (.MeshSize (Utilities|Struct|BreakS_GridShapeData (CallFunction|GetCurrentShapeData))))))
      ;[1 0.5516 0.9945] spawns instanced static mesh via world space
      (Class|InstancedStaticMeshComponent|AddInstanceWorldSpace (Variables|Default|GetInstancedStaticMesh) (LocalVariables|GettileTransform)))))

(fn GetCurrentShapeData
  (bind _grid_shape (Variables|Default|GetGrid%20Shape))
  (bind _returnvalue (Utilities|String|EnumtoString _grid_shape))
  (bind _returnvalue_2 (Utilities|GetDataTableRow "/Game/Blueprints/Core/Grid/GridShapes/DT_GridShapeData.DT_GridShapeData" (Utilities|String|StringToName _returnvalue))
    (:then
      (return _returnvalue_2))
    (:RowNotFound
      (Development|PrintString _returnvalue true true "(R=0.635417,G=0.000000,B=0.005618,A=1.000000)" 5.0))))

(fn DestroyGrid
  (Components|InstancedStaticMesh|ClearInstances (Variables|Default|GetInstancedStaticMesh)))

(fn CalculateCenterandButtomLeft
  (bind _grid_tile_count (Variables|Default|GetGrid%20Tile%20Count))
  (switch Utilities|FlowControl|Switch|SwitchonE_GridShape (Variables|Default|GetGrid%20Shape)
    (:NewEnumerator1
      (LocalVariables|SetC (CallFunction|SnapVectortoVector (Variables|Default|GetGrid%20Center%20Location) (Variables|Default|GetGrid%20Tile%20Size)))
      (return (LocalVariables|GetC) (- (LocalVariables|GetC) (Math|Conversions|ToVector(Vector2D) (* (/ (- (Variables|Default|GetGrid%20Tile%20Count) (Math|Vector2D|MakeVector2D (Math|Float|SelectFloat 0.0 1.0 (CallFunction|IsFloatEven (.x _grid_tile_count))) (Math|Float|SelectFloat 0.0 1.0 (CallFunction|IsFloatEven (.y _grid_tile_count))))) 2.0) (Math|Conversions|ToVector2D(Vector) (Variables|Default|GetGrid%20Tile%20Size)))))))
    (:NewEnumerator3
      (LocalVariables|SetC (CallFunction|SnapVectortoVector (Variables|Default|GetGrid%20Center%20Location) (* (Variables|Default|GetGrid%20Tile%20Size) "2.000000,1.000000,1.000000")))
      (return (LocalVariables|GetC) (- (LocalVariables|GetC) (CallFunction|SnapVectortoVector (Math|Conversions|ToVector(Vector2D) (* (/ (- (Variables|Default|GetGrid%20Tile%20Count) (Math|Vector2D|MakeVector2D 1.0 1.0)) "(X=2.000000,Y=4.000000)") (Math|Conversions|ToVector2D(Vector) (Variables|Default|GetGrid%20Tile%20Size)))) (* (Variables|Default|GetGrid%20Tile%20Size) "2.000000,1.000000,1.000000")))))))

(fn GetTileRotationfromGridIndex
  (params (GridIndex :type Vector%202D%20Structure))
  ;[1 0.302 0.312 1 13] rotates tiles 180° if Grid index is even
  (if (Utilities|Enum|Equal(Enum) (Variables|Default|GetGrid%20Shape) "NewEnumerator3")
    (return (Math|Rotator|MakeRotator 0.0 0.0 (+ (Math|Float|SelectFloat 1.8e+02 0.0 (CallFunction|IsFloatEven (.x GridIndex))) (Math|Float|SelectFloat 1.8e+02 0.0 (CallFunction|IsFloatEven (.y GridIndex))))))
    (else
      ;[1 0.4506 0.1661 1 13] return 0 if Tile is not Triangle
      (return ""))))

(fn GetTileLocationfromGridIndex
  (params (GridIndex :type Vector%202D%20Structure))
  (return (+ (Variables|Default|GetgridBottomLeftCornerLocation) (* (Variables|Default|GetGrid%20Tile%20Size) (Math|Conversions|ToVector(Vector2D) (* GridIndex (Utilities|Select :Index (Variables|Default|GetGrid%20Shape) :NewEnumerator0 "" :NewEnumerator1 "(X=1.000000,Y=1.000000)" :NewEnumerator2 "(X=1.000000,Y=1.000000)" :NewEnumerator3 "(X=1.000000,Y=0.500000)")))))))